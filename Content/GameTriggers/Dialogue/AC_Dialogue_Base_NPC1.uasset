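; Dialogue component for the Cloak NPC, who welcomes the player to Nephraim and grants entry through its gates.
; It overrides Dialogue, switching on DialogueTreeIndex and nesting AddDialogue calls that branch on the chosen option.
; Accepting entry advances the tree index and plays the Door_Open level sequence, while declining or staying silent closes the conversation without advancing it.
; Later conversations show a random go-in line, then clear dialogue progress.
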(fn `Dialogue`
  (`parent.Dialogue`)
  (switch `int` (`self.DialogueTreeIndex`)
    (:`0`
      (bind (_state _optionindex) (`self.AddDialogue` "Cloak" "Hello, weary traveller." (`|MakeArray` "Hello!" "..." :!type "Text")))
      (switch `/Game/GameTriggers/Dialogue/Enum_DialogueState` _state
        (:`NewEnumerator0`
          (switch `int` _optionindex
            (:`0`
              (bind (_state_2 _optionindex_2) (`self.AddDialogue` "Cloak" "Welcome to the land of Nephraim." (`|MakeArray` "Thank you!" "..." :!type "Text")))
              (switch `/Game/GameTriggers/Dialogue/Enum_DialogueState` _state_2
                (:`NewEnumerator0`
                  (switch `int` _optionindex_2
                    (:`0`
                      (bind (_state_3 _optionindex_3) (`self.AddDialogue` "Cloak" "Would you like to enter Nephraim?" (`|MakeArray` "Yes." "No." :!type "Text")))
                      (switch `/Game/GameTriggers/Dialogue/Enum_DialogueState` _state_3
                        (:`NewEnumerator0`
                          (switch `int` _optionindex_3
                            (:`0`
                              (bind _state_4 (`self.AddDialogue` "Cloak" "You are free to enter the gates when you wish. " (`|MakeArray` "Finish" :!type "Text")))
                              (switch `/Game/GameTriggers/Dialogue/Enum_DialogueState` _state_4
                                (:`NewEnumerator0`
                                  (set `self.DialogueTreeIndex` 1)
                                  (`self.CloseConversation`)
                                  (bind _outactor (`LevelSequencePlayer.CreateLevelSequencePlayer` "/Game/GameTriggers/Triggers/Door_Open.Door_Open" (make `MovieSceneSequencePlaybackSettings` false (make `MovieSceneSequenceLoopCount` -1))))
                                  (`MovieSceneSequencePlayer.Play` (`LevelSequenceActor.SequencePlayer` _outactor)))))
                            (:`1`
                              (`self.RemoveDialogueProgress` 0)
                              (`self.CloseConversation`))))))
                    (:`1`
                      (bind _state_5 (`self.AddDialogue` "Cloak" "Okay, are you going to talk?" (`|MakeArray` "No." :!type "Text")))
                      (switch `/Game/GameTriggers/Dialogue/Enum_DialogueState` _state_5
                        (:`NewEnumerator0`
                          (`self.RemoveDialogueProgress` 0)
                          (`self.CloseConversation`))))))))
            (:`1`
              (bind _state_6 (`self.AddDialogue` "Cloak" "Okay, are you going to talk?" (`|MakeArray` "No." :!type "Text")))
              (switch `/Game/GameTriggers/Dialogue/Enum_DialogueState` _state_6
                (:`NewEnumerator0`
                  (set `self.DialogueTreeIndex` 0)
                  (`self.CloseConversation`))))))))
    (:`1`
      (bind _state_7 (`self.AddDialogue` "Cloak" (select `int` (`KismetMathLibrary.RandomIntegerInRange` 0 2) :`0` "You are free to enter." :`1` "Go in, please." :`2` "Time waits for no one!" :!type "Text") (`|MakeArray` "Finish" :!type "Text")))
      (switch `/Game/GameTriggers/Dialogue/Enum_DialogueState` _state_7
        (:`NewEnumerator0`
          (`self.ClearDialogueProgress`)
          (`self.CloseConversation`))))))