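; Dialogue component for the Angry Villager NPC, who complains about heretics clashing with the Cloakhood and stealing Cog Fire.
; Overrides Dialogue, calls the parent, then builds a branching tree of AddDialogue calls gated on Passthrough state and chosen option index.
; The first choice leads through lore about Cog Fire wisps in a nearby Orb, while the second provokes an accusation of heresy.
; Both branches end by clearing dialogue progress and closing the conversation.
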(fn `Dialogue`
  (`parent.Dialogue`)
  (bind (_state _optionindex) (`self.AddDialogue` "Angry Villager" "The heretics have been at it again!" (`|MakeArray` "What happened?" "Are you a heretic?" :!type "Text")))
  (switch `/Game/GameTriggers/Dialogue/Enum_DialogueState` _state
    (:`NewEnumerator0`
      (switch `int` _optionindex
        (:`0`
          (bind (_state_2 _optionindex_2) (`self.AddDialogue` "Angry Villager" "Oh, those things with the heretics?" (`|MakeArray` "Continue" :!type "Text")))
          (switch `/Game/GameTriggers/Dialogue/Enum_DialogueState` _state_2
            (:`NewEnumerator0`
              (switch `int` _optionindex_2
                (:`0`
                  (bind (_state_3 _optionindex_3) (`self.AddDialogue` "Angry Villager" "They've been clashing with 'em Cloakhood..." (`|MakeArray` "Continue" :!type "Text")))
                  (switch `/Game/GameTriggers/Dialogue/Enum_DialogueState` _state_3
                    (:`NewEnumerator0`
                      (switch `int` _optionindex_3
                        (:`0`
                          (bind (_state_4 _optionindex_4) (`self.AddDialogue` "Angry Villager" "And stealing their Cog Fire." (`|MakeArray` "Cog Fire?" :!type "Text")))
                          (switch `/Game/GameTriggers/Dialogue/Enum_DialogueState` _state_4
                            (:`NewEnumerator0`
                              (switch `int` _optionindex_4
                                (:`0`
                                  (bind (_state_5 _optionindex_5) (`self.AddDialogue` "Angry Villager" "Those little wispy guys that pop up sometimes." (`|MakeArray` "Continue" :!type "Text")))
                                  (switch `/Game/GameTriggers/Dialogue/Enum_DialogueState` _state_5
                                    (:`NewEnumerator0`
                                      (switch `int` _optionindex_5
                                        (:`0`
                                          (bind _state_6 (`self.AddDialogue` "Angry Villager" "There's a bunch of 'em in that Orb down there." (`|MakeArray` "Finish" :!type "Text")))
                                          (switch `/Game/GameTriggers/Dialogue/Enum_DialogueState` _state_6
                                            (:`NewEnumerator0`
                                              (`self.ClearDialogueProgress`)
                                              (`self.CloseConversation`))))))))))))))))))))
        (:`1`
          (bind (_state_7 _optionindex_6) (`self.AddDialogue` "Angry Villager" "What kind of BLASPHEMY is that??" (`|MakeArray` "Continue" :!type "Text")))
          (switch `/Game/GameTriggers/Dialogue/Enum_DialogueState` _state_7
            (:`NewEnumerator0`
              (switch `int` _optionindex_6
                (:`0`
                  (bind _state_8 (`self.AddDialogue` "Angry Villager" "YOU are the heretic here!!" (`|MakeArray` "Finish" :!type "Text")))
                  (switch `/Game/GameTriggers/Dialogue/Enum_DialogueState` _state_8
                    (:`NewEnumerator0`
                      (`self.ClearDialogueProgress`)
                      (`self.CloseConversation`))))))))))))