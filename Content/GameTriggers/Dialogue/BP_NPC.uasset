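; BP_NPC is a dialogue NPC actor that displays its character name and reports to its interactor when a conversation ends.
; The construction script writes CharacterName into the TxtCharacterName component.
; SetInteractableState shows or hides that name label based on whether interaction is available.
; ConversationCloses forwards the closing notification to InteractInstigator through ConversationClosesMessage.
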(event `/Game/GameTriggers/Dialogue/BPI_Interactable.SetInteractableState`
  (params (`CanShowInter??` :type Boolean))
  (if `CanShowInter??`
    (`SceneComponent.SetVisibility` (`self.Txt_CharacterName`) true false)
    (else
      (`SceneComponent.SetVisibility` (`self.Txt_CharacterName`) false false))))

(event `/Game/GameTriggers/Dialogue/BPI_Interactable.ConversationCloses`
  (message `/Game/GameTriggers/Dialogue/BPI_Interactable.ConversationCloses` (`self.InteractInstigator`)))

(fn `UserConstructionScript`
  (`TextRenderComponent.K2_SetText` (`self.Txt_CharacterName`) (`self.CharacterName`)))