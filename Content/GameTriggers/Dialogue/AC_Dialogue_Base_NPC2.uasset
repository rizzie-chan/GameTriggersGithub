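; Dialogue component for a villager NPC who complains about the bad air, with one two-way player choice at the start.
; Overrides Dialogue, calls the parent, then chains AddDialogue nodes that branch on option index whenever their state is Passthrough.
; Agreeing leads to talk of the Cloakhood's Orb of Light and free gate entry, while doubting leads to an allergy aside.
; Both branches end by clearing dialogue progress and closing the conversation.
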(fn `Dialogue`
  (`parent.Dialogue`)
  (bind (_state _optionindex) (`self.AddDialogue` "Villager" "The air hasn't been good in here recently." (`|MakeArray` "Stifling, for sure." "Are you sure?" :!type "Text")))
  (switch `/Game/GameTriggers/Dialogue/Enum_DialogueState` _state
    (:`NewEnumerator0`
      (switch `int` _optionindex
        (:`0`
          (bind (_state_2 _optionindex_2) (`self.AddDialogue` "Villager" "Glad you understand me." (`|MakeArray` "Continue" :!type "Text")))
          (switch `/Game/GameTriggers/Dialogue/Enum_DialogueState` _state_2
            (:`NewEnumerator0`
              (switch `int` _optionindex_2
                (:`0`
                  (bind (_state_3 _optionindex_3) (`self.AddDialogue` "Villager" "That new Obr of Light..." (`|MakeArray` "Continue" :!type "Text")))
                  (switch `/Game/GameTriggers/Dialogue/Enum_DialogueState` _state_3
                    (:`NewEnumerator0`
                      (switch `int` _optionindex_3
                        (:`0`
                          (bind (_state_4 _optionindex_4) (`self.AddDialogue` "Villager" "You know, the one the Cloakhood installed?" (`|MakeArray` "Continue" :!type "Text")))
                          (switch `/Game/GameTriggers/Dialogue/Enum_DialogueState` _state_4
                            (:`NewEnumerator0`
                              (switch `int` _optionindex_4
                                (:`0`
                                  (bind (_state_5 _optionindex_5) (`self.AddDialogue` "Villager" "It's making people go a bit..." (`|MakeArray` "Continue" :!type "Text")))
                                  (switch `/Game/GameTriggers/Dialogue/Enum_DialogueState` _state_5
                                    (:`NewEnumerator0`
                                      (switch `int` _optionindex_5
                                        (:`0`
                                          (bind (_state_6 _optionindex_6) (`self.AddDialogue` "Villlager" "Off their knockers." (`|MakeArray` "Continue" :!type "Text")))
                                          (switch `/Game/GameTriggers/Dialogue/Enum_DialogueState` _state_6
                                            (:`NewEnumerator0`
                                              (switch `int` _optionindex_6
                                                (:`0`
                                                  (bind (_state_7 _optionindex_7) (`self.AddDialogue` "Villager" "Maybe the heretics will get rid of it." (`|MakeArray` "Continue" :!type "Text")))
                                                  (switch `/Game/GameTriggers/Dialogue/Enum_DialogueState` _state_7
                                                    (:`NewEnumerator0`
                                                      (switch `int` _optionindex_7
                                                        (:`0`
                                                          (bind _state_8 (`self.AddDialogue` "Villager" "You are free to enter the gates when you wish. " (`|MakeArray` "Finish" :!type "Text")))
                                                          (switch `/Game/GameTriggers/Dialogue/Enum_DialogueState` _state_8
                                                            (:`NewEnumerator0`
                                                              (`self.ClearDialogueProgress`)
                                                              (`self.CloseConversation`))))))))))))))))))))))))))))
        (:`1`
          (bind (_state_9 _optionindex_8) (`self.AddDialogue` "Villager" "*sniffles*" (`|MakeArray` "Continue" :!type "Text")))
          (switch `/Game/GameTriggers/Dialogue/Enum_DialogueState` _state_9
            (:`NewEnumerator0`
              (switch `int` _optionindex_8
                (:`0`
                  (bind (_state_10 _optionindex_9) (`self.AddDialogue` "Villager" "Hm, maybe just my allergies." (`|MakeArray` "Continue" :!type "Text")))
                  (switch `/Game/GameTriggers/Dialogue/Enum_DialogueState` _state_10
                    (:`NewEnumerator0`
                      (switch `int` _optionindex_9
                        (:`0`
                          (bind _state_11 (`self.AddDialogue` "Villager" "Those goddamn dust spores." (`|MakeArray` "Finish" :!type "Text")))
                          (switch `/Game/GameTriggers/Dialogue/Enum_DialogueState` _state_11
                            (:`NewEnumerator0`
                              (`self.ClearDialogueProgress`)
                              (`self.CloseConversation`))))))))))))))))