(fn `Dialogue`
  (`parent.Dialogue`)
  (bind (_state _optionindex) (`self.AddDialogue` "Child" "Excuseeee me..." (`|MakeArray` "???" "What do you want?" :!type "Text")))
  (switch `/Game/GameTriggers/Dialogue/Enum_DialogueState` _state
    (:`NewEnumerator0`
      (switch `int` _optionindex
        (:`0`
          _)
        (:`1`
          _))
      (bind (_state_2 _optionindex_2) (`self.AddDialogue` "Child" "My ma says not to approach the Orb of Light at night..." (`|MakeArray` "Continue" :!type "Text")))
      (switch `/Game/GameTriggers/Dialogue/Enum_DialogueState` _state_2
        (:`NewEnumerator0`
          (switch `int` _optionindex_2
            (:`0`
              (bind (_state_3 _optionindex_3) (`self.AddDialogue` "Child" "Apparently it swallows children whole!" (`|MakeArray` "What is the Orb of Light?" "Your mom says a lot." :!type "Text")))
              (switch `/Game/GameTriggers/Dialogue/Enum_DialogueState` _state_3
                (:`NewEnumerator0`
                  (switch `int` _optionindex_3
                    (:`0`
                      (bind (_state_4 _optionindex_4) (`self.AddDialogue` "Child" "My ma says it is the juxtaposition of darkness!" (`|MakeArray` "What's the juxtaposition of darkness?" "Your mom says a lot." :!type "Text")))
                      (switch `/Game/GameTriggers/Dialogue/Enum_DialogueState` _state_4
                        (:`NewEnumerator0`
                          (switch `int` _optionindex_4
                            (:`0`
                              (bind (_state_5 _optionindex_5) (`self.AddDialogue` "Child" "But only in the daytime!" (`|MakeArray` "Continue" :!type "Text")))
                              (switch `/Game/GameTriggers/Dialogue/Enum_DialogueState` _state_5
                                (:`NewEnumerator0`
                                  (switch `int` _optionindex_5
                                    (:`0`
                                      (bind (_state_6 _optionindex_6) (`self.AddDialogue` "Child" "My ma says that at night..." (`|MakeArray` "Continue" :!type "Text")))
                                      (switch `/Game/GameTriggers/Dialogue/Enum_DialogueState` _state_6
                                        (:`NewEnumerator0`
                                          (switch `int` _optionindex_6
                                            (:`0`
                                              (bind (_state_7 _optionindex_7) (`self.AddDialogue` "Child" "it becomes the juxtaposition of light. " (`|MakeArray` "You're not making a lot of sense..." "Your mom says a lot. " :!type "Text")))
                                              (switch `/Game/GameTriggers/Dialogue/Enum_DialogueState` _state_7
                                                (:`NewEnumerator0`
                                                  (switch `int` _optionindex_7
                                                    (:`0`
                                                      (bind _state_8 (`self.AddDialogue` "Child" "Your mom isn't making a lot of sense!" (`|MakeArray` "Finish" :!type "Text")))
                                                      (switch `/Game/GameTriggers/Dialogue/Enum_DialogueState` _state_8
                                                        (:`NewEnumerator0`
                                                          (`self.ClearDialogueProgress`)
                                                          (`self.CloseConversation`))))
                                                    (:`1`
                                                      (bind _state_9 (`self.AddDialogue` "Child" "Your mom is disappointed that she birthed you." (`|MakeArray` "Finish" :!type "Text")))
                                                      (switch `/Game/GameTriggers/Dialogue/Enum_DialogueState` _state_9
                                                        (:`NewEnumerator0`
                                                          (`self.ClearDialogueProgress`)
                                                          (`self.CloseConversation`))))))))))))))))
                            (:`1`
                              (bind _state_10 (`self.AddDialogue` "Child" "Your mom is disappointed that she birthed you." (`|MakeArray` "Finish" :!type "Text")))
                              (switch `/Game/GameTriggers/Dialogue/Enum_DialogueState` _state_10
                                (:`NewEnumerator0`
                                  (`self.ClearDialogueProgress`)
                                  (`self.CloseConversation`))))))))
                    (:`1`
                      (bind _state_11 (`self.AddDialogue` "Child" "Your mom is disappointed that she birthed you." (`|MakeArray` "Finish" :!type "Text")))
                      (switch `/Game/GameTriggers/Dialogue/Enum_DialogueState` _state_11
                        (:`NewEnumerator0`
                          (`self.ClearDialogueProgress`)
                          (`self.CloseConversation`))))))))))))))